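; BP_Box_Counter is an actor that tracks how many breakable boxes remain in the level.
; On BeginPlay it counts all BP_Breakable_Box actors, storing that count as both the total and the remaining value.
; Its BoxBroken event decrements the remaining count behind a non-negative check.
; Both steps report the numbers through on-screen debug prints.
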(event Custom|Box%20Broken
  (if (>= (Variables|Default|GetBoxesRemaining) 0)
    (bind _output_get (Variables|Default|SetBoxesRemaining (- (Variables|Default|GetBoxesRemaining) 1)))
    (Development|PrintString (Utilities|String|Append "Boxes Remaining: " (Utilities|String|ToString(Integer) _output_get)) true true "(R=0.000000,G=0.660000,B=1.000000,A=1.000000)" 5.0)))

(event EventBeginPlay
  (bind _outactors (Actor|GetAllActorsOfClass "/Game/Game/Blueprints/BP_Breakable_Box.BP_Breakable_Box_C"))
  (bind _output_get (Variables|Default|SetTotalBoxes (Utilities|Array|Length _outactors)))
  (Variables|Default|SetBoxesRemaining (Utilities|Array|Length _outactors))
  (Development|PrintString (Utilities|String|Append "Total boxes: " (Utilities|String|ToString(Integer) _output_get)) true true "(R=0.000000,G=0.660000,B=1.000000,A=1.000000)" 5.0))

(event Collision|EventActorBeginOverlap
  (params (OtherActor :type Actor%20Object%20Reference)))

(event EventTick
  (params (DeltaSeconds :type Float%20%28single-precision%29)))

(fn ConstructionScript)