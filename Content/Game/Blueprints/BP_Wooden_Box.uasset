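; BP_Wooden_Box is a child Blueprint for a breakable wooden box that reacts to a bounce action.
; Its BounceAction override runs the parent behavior, plays the VR_grab sound at reduced volume, then calls BreakBox.
; BreakBox is not defined in this graph, and the construction script only calls the parent.
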(event EventBeginPlay
  (|CallParentFunction) ; This node is disabled and will not be called.\nDrag off pins to build functionality.
)

(event Collision|EventActorBeginOverlap
  (params (OtherActor :type Actor%20Object%20Reference))
  (|CallParentFunction OtherActor) ; This node is disabled and will not be called.\nDrag off pins to build functionality.
)

(event EventTick
  (params (DeltaSeconds :type Float%20%28single-precision%29))
  (|CallParentFunction DeltaSeconds) ; This node is disabled and will not be called.\nDrag off pins to build functionality.
)

(event EventBounceAction
  (|CallParentFunction)
  (Audio|PlaySoundatLocation "/Engine/VREditor/Sounds/VR_grab.VR_grab" "0, 0, 0" "0, 0, 0" 0.5 1.0 0.0 0 0 0 0)
  (CallFunction|BreakBox))

(fn ConstructionScript
  (|CallParentFunction))