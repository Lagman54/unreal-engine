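; BP_Breakable_Box is a box that can be broken, reporting its destruction to a box counter in the level.
; On BeginPlay it finds the BP_Box_Counter with GetActorOfClass and caches the reference.
; BreakBox destroys the actor, then calls BoxBroken on that counter.
; Nothing in this Blueprint calls BreakBox, and its Tick and overlap events are disabled.
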(event EventBeginPlay
  (|CallParentFunction)
  (bind _returnvalue (Actor|GetActorOfClass "/Game/Game/Blueprints/BP_Box_Counter.BP_Box_Counter_C"))
  (Variables|Default|SetBoxCounter _returnvalue))

(event Collision|EventActorBeginOverlap
  (params (OtherActor :type Actor%20Object%20Reference))
  (|CallParentFunction OtherActor) ; This node is disabled and will not be called.\nDrag off pins to build functionality.
)

(event EventTick
  (params (DeltaSeconds :type Float%20%28single-precision%29))
  (|CallParentFunction DeltaSeconds) ; This node is disabled and will not be called.\nDrag off pins to build functionality.
)

(fn ConstructionScript
  (|CallParentFunction))

(fn BreakBox
  (Actor|DestroyActor)
  (Default|BoxBroken (Variables|Default|GetBoxCounter)))