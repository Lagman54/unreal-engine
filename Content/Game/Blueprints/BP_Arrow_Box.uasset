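; BP_Arrow_Box is a box actor with a bounce trigger on top, set up to launch upward.
; On BeginPlay it casts the TopBounceTrigger child actor to BP_Bounce_Trigger and overrides its LaunchVelocity with a fixed vertical value.
; The launch itself is left to that trigger, as overlap and tick events here are disabled and the construction script only calls the parent.
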(event EventBeginPlay
  (bind _asbp_bounce_trigger (Utilities|Casting|CastToBP_Bounce_Trigger (Variables|/Script/Engine.ChildActorComponent|GetChildActor (Variables|Default|GetTop%20Bounce%20Trigger))))
  (Class|KismetMathLibrary|VectorSet (Variables|/Game/Game/Blueprints/BP_Bounce_Trigger.BP_Bounce_Trigger_C|GetLaunch%20Velocity _asbp_bounce_trigger) 0.0 0.0 1e+03))

(event Collision|EventActorBeginOverlap
  (params (OtherActor :type Actor%20Object%20Reference))
  (|CallParentFunction OtherActor) ; Этот узел отключен и не будет вызываться.\nПеретащите контакты, чтобы построить функционал.
)

(event EventTick
  (params (DeltaSeconds :type Float%20%28single-precision%29))
  (|CallParentFunction DeltaSeconds) ; Этот узел отключен и не будет вызываться.\nПеретащите контакты, чтобы построить функционал.
)

(fn ConstructionScript
  (|CallParentFunction))