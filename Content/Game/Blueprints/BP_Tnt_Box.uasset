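; TNT crate, a child of a breakable box Blueprint, that starts a countdown when bounced on and then explodes.
; BounceAction calls the parent behavior, then StartTimer uses a flag to ignore repeat triggers and sets a looping one-second timer on UpdateTimer.
; UpdateTimer shows the remaining count on four text renders and decrements it.
; At zero, TimerCompleted spawns the explosion effect and sound, then calls BreakBox.
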(event Custom|TimerCompleted
  (bind _returnvalue (Transformation|GetActorLocation))
  (Effects|SpawnEmitteratLocation "/Game/StarterContent/Particles/P_Explosion.P_Explosion" _returnvalue "0, 0, 0" "5.000000,5.000000,5.000000" false)
  (Audio|PlaySoundatLocation "/Game/StarterContent/Audio/Explosion01.Explosion01" _returnvalue "0, 0, 0" 0.5 1.0 0.0 0 0 0 0)
  (CallFunction|BreakBox)
  (Development|PrintString "Boom!"))

(event EventBeginPlay
  (|CallParentFunction) ; This node is disabled and will not be called.\nDrag off pins to build functionality.
)

(event Collision|EventActorBeginOverlap
  (params (OtherActor :type Actor%20Object%20Reference))
  (|CallParentFunction OtherActor) ; This node is disabled and will not be called.\nDrag off pins to build functionality.
)

(event EventTick
  (params (DeltaSeconds :type Float%20%28single-precision%29))
  (|CallParentFunction DeltaSeconds) ; This node is disabled and will not be called.\nDrag off pins to build functionality.
)

(event EventBounceAction
  (|CallParentFunction)
  (CallFunction|StartTimer))

(fn ConstructionScript
  (|CallParentFunction))

(fn StartTimer
  (if (not (Variables|Default|GetisTimerRunning))
    (bind _output_get (Variables|Default|SetisTimerRunning true))
    (Development|PrintString "Timer Started")
    (CallFunction|UpdateTimer)
    (Utilities|Time|SetTimerbyFunctionName 0 "UpdateTimer" 1.0 _output_get)))

(fn UpdateTimer
  (if (!= (Variables|Default|GettntTimer) 0)
    (Rendering|Components|TextRender|SetText (Variables|Default|GetTextRender) (Utilities|Text|ToText(Integer) (Variables|Default|GettntTimer)))
    (Rendering|Components|TextRender|SetText (Variables|Default|GetTextRender1) (Utilities|Text|ToText(Integer) (Variables|Default|GettntTimer)))
    (Rendering|Components|TextRender|SetText (Variables|Default|GetTextRender2) (Utilities|Text|ToText(Integer) (Variables|Default|GettntTimer)))
    (Rendering|Components|TextRender|SetText (Variables|Default|GetTextRender3) (Utilities|Text|ToText(Integer) (Variables|Default|GettntTimer))))
  (if (> (Variables|Default|GettntTimer) 0)
    (Variables|Default|SettntTimer (- (Variables|Default|GettntTimer) 1))
    (else
      (Variables|Default|SetisTimerRunning false)
      (CallFunction|TimerCompleted))))