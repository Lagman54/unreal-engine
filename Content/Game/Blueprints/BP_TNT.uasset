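; BP_TNT is an explosive crate that bounces the player upward and then blows itself up.
; A hit on TntBox with an exactly downward impact normal launches the third-person character straight up.
; After a short delay it spawns a scaled-up explosion emitter, plays a sound and destroys itself.
; The explosion applies no damage, and debug strings print at the bounce and the blast.
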(event OnComponentHit(TntBox)
  (params (HitComponent :type Primitive%20Component%20Object%20Reference) (OtherActor :type Actor%20Object%20Reference) (OtherComp :type Primitive%20Component%20Object%20Reference) (NormalImpulse :type Vector :default "0, 0, 0") (Hit :type Hit%20Result%20Structure%20%28by%20ref%29))
  (bind _returnvalue (Transformation|GetActorLocation))
  (if (Utilities|Operators|EqualEqual (.ImpactNormal (Collision|BreakHitResult Hit)) "0.000000,0.000000,-1.000000" 0.0)
    (bind _asbp_third_person_character (Utilities|Casting|CastToBP_ThirdPersonCharacter OtherActor))
    (Character|LaunchCharacter _asbp_third_person_character "0.000000,0.000000,600.000000" false false)
    (Development|PrintString "Bounce")
    (Utilities|FlowControl|Delay 3.0)
    (Effects|SpawnEmitteratLocation "/Game/StarterContent/Particles/P_Explosion.P_Explosion" _returnvalue "0, 0, 0" "5.000000,5.000000,5.000000" false)
    (Audio|PlaySoundatLocation "/Game/StarterContent/Audio/Explosion01.Explosion01" _returnvalue "0, 0, 0" 1.0 1.0 0.0 0 0 0 0)
    (Actor|DestroyActor)
    (Development|PrintString "Boom!")))

(event EventBeginPlay)

(event Collision|EventActorBeginOverlap
  (params (OtherActor :type Actor%20Object%20Reference)))

(event EventTick
  (params (DeltaSeconds :type Float%20%28single-precision%29)))

(fn ConstructionScript)